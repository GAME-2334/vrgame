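; BP_WB_DoorLock_1 is a door lock actor that slides vertically by a Drop offset once triggered.
; StartTick fires only once through a DoOnce, caching the starting location and setting IsOpening.
; Tick then eases Z toward the offset target with FInterpTo, stopping and printing the location when Z is at or above it.
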(event `StartTick`
  (`/Engine/EditorBlueprintResources/StandardMacros.DoOnce` false
    (:`Completed`
      (set `self.location` (`self.K2_GetActorLocation`))
      (set `self.isOpening` true))))

(event `self.ReceiveTick`
  (params (DeltaSeconds :type "Float (single-precision)"))
  (bind (_returnvalue_x _returnvalue_y _returnvalue_z) (`KismetMathLibrary.BreakVector` (`self.K2_GetActorLocation`)))
  (bind _returnvalue (`self.K2_GetActorLocation`))
  (bind (_location_x _location_y) (`KismetMathLibrary.BreakVector` (`self.location`)))
  (bind (_location_x_2 _location_y_2 _location_z) (`KismetMathLibrary.BreakVector` (`self.location`)))
  (bind (_location_x_3 _location_y_3 _location_z_2) (`KismetMathLibrary.BreakVector` (`self.location`)))
  (if (`self.isOpening`)
    (`self.K2_SetActorLocation` (`KismetMathLibrary.MakeVector` _location_x _location_y (`KismetMathLibrary.FInterpTo` _returnvalue_z (+ _location_z_2 (`self.Drop`)) DeltaSeconds 1.0)))
    (bind _output_get (set `self.newlocation` _returnvalue))
    (if (>= (.z _output_get) (+ _location_z (`self.Drop`)))
      (set `self.isOpening` false)
      (`KismetSystemLibrary.PrintString` (`KismetStringLibrary.Conv_VectorToString` _returnvalue)))))

(fn `UserConstructionScript`)