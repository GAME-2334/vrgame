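; BP_WB_DoorLock_2 is a World Builder door-lock actor that lowers itself once when something overlaps its Box trigger.
; The first overlap, with no filter on the overlapping actor, passes a DoOnce, caches the actor's location and sets IsDropping.
; Tick then eases Z toward the start height minus Drop with FInterpTo, clearing the flag once that height is reached.
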(event `self.Box.OnComponentBeginOverlap`
  (params (OverlappedComponent :type "PrimitiveComponent Object Reference") (OtherActor :type "Actor Object Reference") (OtherComp :type "PrimitiveComponent Object Reference") (OtherBodyIndex :type Integer) (bFromSweep :type Boolean) (SweepResult :type "HitResult Structure (by ref)"))
  (`/Engine/EditorBlueprintResources/StandardMacros.DoOnce` false
    (:`Completed`
      (set `self.location` (`self.K2_GetActorLocation`))
      (set `self.isDropping` true))))

(event `self.ReceiveTick`
  (params (DeltaSeconds :type "Float (single-precision)"))
  (bind (_returnvalue_x _returnvalue_y _returnvalue_z) (`KismetMathLibrary.BreakVector` (`self.K2_GetActorLocation`)))
  (bind (_location_x _location_y) (`KismetMathLibrary.BreakVector` (`self.location`)))
  (bind (_location_x_2 _location_y_2 _location_z) (`KismetMathLibrary.BreakVector` (`self.location`)))
  (bind (_location_x_3 _location_y_3 _location_z_2) (`KismetMathLibrary.BreakVector` (`self.location`)))
  (if (`self.isDropping`)
    (`self.K2_SetActorLocation` (`KismetMathLibrary.MakeVector` _location_x _location_y (`KismetMathLibrary.FInterpTo` _returnvalue_z (- _location_z_2 (`self.Drop`)) DeltaSeconds 1.0)))
    (bind _output_get (set `self.newlocation` (`self.K2_GetActorLocation`)))
    (if (<= (.z _output_get) (- _location_z (`self.Drop`)))
      (set `self.isDropping` false))))

(fn `UserConstructionScript`)