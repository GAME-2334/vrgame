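; BP_WB_DoorLockRegular2 is a World Builder door lock that slides vertically with a sliding sound.
; StartTick raises it by Drop; the first Box overlap snaps it to the raised height, then lowers it by Drop2.
; Tick drives both moves with FInterpTo, and Box1 resets the attached switch after a drop.
; Both moves are DoOnce-gated; Reset is empty and the gate resets are unwired.
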(event `self.ReceiveBeginPlay`
  (set `self.startinglocation` (`self.K2_GetActorLocation`)))

(event `StartTick`
  (`/Engine/EditorBlueprintResources/StandardMacros.DoOnce` false
    (:`Completed`
      (set `self.location` (`self.K2_GetActorLocation`))
      (set `self.isOpening` true)
      (`GameplayStatics.PlaySoundAtLocation` (`self.sliding sound`) (`self.K2_GetActorLocation`) (struct) 1.0 1.0 0.0 null null null))))

(event `self.ReceiveTick`
  (params (DeltaSeconds :type "Float (single-precision)"))
  (bind (_returnvalue_x _returnvalue_y _returnvalue_z) (`KismetMathLibrary.BreakVector` (`self.K2_GetActorLocation`)))
  (bind (_returnvalue_x_2 _returnvalue_y_2 _returnvalue_z_2) (`KismetMathLibrary.BreakVector` (`self.K2_GetActorLocation`)))
  (bind (_location_x _location_y _location_z) (`KismetMathLibrary.BreakVector` (`self.location`)))
  (bind (_location_x_2 _location_y_2) (`KismetMathLibrary.BreakVector` (`self.location`)))
  (bind (_location_x_3 _location_y_3 _location_z_2) (`KismetMathLibrary.BreakVector` (`self.location`)))
  (bind (_location_x_4 _location_y_4 _location_z_3) (`KismetMathLibrary.BreakVector` (`self.location`)))
  (bind (_location_x_5 _location_y_5) (`KismetMathLibrary.BreakVector` (`self.location`)))
  (bind (_location_x_6 _location_y_6 _location_z_4) (`KismetMathLibrary.BreakVector` (`self.location`)))
  (`|ExecutionSequence`
    (:`then_0`
      (if (`self.isOpening`)
        (if (not (`self.isDropping`))
          (`self.K2_SetActorLocation` (`KismetMathLibrary.MakeVector` _location_x_5 _location_y_5 (`KismetMathLibrary.FInterpTo` _returnvalue_z_2 (+ _location_z_4 (`self.Drop`)) DeltaSeconds 1.0)))
          (bind _output_get (set `self.newlocation` (`self.K2_GetActorLocation`)))
          (if (>= (.z _output_get) (+ (+ _location_z (`self.Drop`)) -2.0))
            (set `self.isOpening` false)))))
    (:`then_1`
      (if (`self.isDropping`)
        (`self.K2_SetActorLocation` (`KismetMathLibrary.MakeVector` _location_x_2 _location_y_2 (`KismetMathLibrary.FInterpTo` _returnvalue_z (- _location_z_3 (`self.Drop2`)) DeltaSeconds 2.0)))
        (bind _output_get_2 (set `self.newlocation` (`self.K2_GetActorLocation`)))
        (if (<= (.z _output_get_2) (+ (- _location_z_2 (`self.Drop2`)) 2.0))
          (set `self.isDropping` false)
          (set `self.isOpening` false))))))

(event `Reset`)

(event `self.Box.OnComponentBeginOverlap`
  (params (OverlappedComponent :type "PrimitiveComponent Object Reference") (OtherActor :type "Actor Object Reference") (OtherComp :type "PrimitiveComponent Object Reference") (OtherBodyIndex :type Integer) (bFromSweep :type Boolean) (SweepResult :type "HitResult Structure (by ref)"))
  (bind (_startinglocation_x _startinglocation_y _startinglocation_z) (`KismetMathLibrary.BreakVector` (`self.startinglocation`)))
  (`/Engine/EditorBlueprintResources/StandardMacros.DoOnce` false
    (:`Completed`
      (`self.K2_SetActorLocation` (`KismetMathLibrary.MakeVector` _startinglocation_x _startinglocation_y (+ _startinglocation_z (`self.Drop`))))
      (set `self.location` (`self.K2_GetActorLocation`))
      (set `self.isDropping` true)
      (`GameplayStatics.PlaySoundAtLocation` (`self.sliding sound`) (`self.K2_GetActorLocation`) (struct) 1.0 1.0 0.0 null null null)
      (set `self.dropped` true))))

(event `self.Box1.OnComponentBeginOverlap`
  (params (OverlappedComponent :type "PrimitiveComponent Object Reference") (OtherActor :type "Actor Object Reference") (OtherComp :type "PrimitiveComponent Object Reference") (OtherBodyIndex :type Integer) (bFromSweep :type Boolean) (SweepResult :type "HitResult Structure (by ref)"))
  (if (`self.dropped`)
    (`/Game/Blueprints/InteractableComponents/SwitchInteractableRegular1.SwitchReset` (`/Game/World_Builder/World_BluePrints/BP_WB_DoorSwitchRegular2.SwitchInteractableRegular1` (`self.attachedSwitch`)))
    (set `self.dropped` false)))

(fn `UserConstructionScript`)