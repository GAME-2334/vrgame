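; Level hook for the second level that gives the desktop or VR player the flashlight and runs an oxygen survival mechanic.
; On BeginPlay it finds or creates the OxygenMeter widget, shows it, starts the oxygen drain and shares the meter reference.
; Tick watches the bar and, when empty, fades the camera out, then opens Level_1 unless oxygen was regained during the fade, in which case it fades back in.
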(event `self.ReceiveBeginPlay`
  (`parent.ReceiveBeginPlay`)
  (if (`self.Is Desktop`)
    (`/Game/FirstPersonBP/Blueprints/FirstPersonCharacter.PickedUpFlashLight` (`self.Desktop Player`))
    (else
      (`/Game/VRTemplate/Blueprints/VRPawn.PickedUpFlashLight` (`self.VR Player`))))
  (bind _foundwidgets (`WidgetBlueprintLibrary.GetAllWidgetsOfClass` "/Game/Oxygen/OxygenMeter.OxygenMeter_C"))
  (bind _output (`|GetArrayItem` _foundwidgets))
  (`/Engine/EditorBlueprintResources/StandardMacros.IsValid` _output
    (:`Is Valid`
      (set `self.Oxygen Meter` _output))
    (:`Is Not Valid`
      (bind _returnvalue (`|GenericCreateObject` "/Game/Oxygen/OxygenMeter.OxygenMeter_C" self))
      (bind _output_get (set `self.Oxygen Meter` _returnvalue))))
  (`UserWidget.AddToViewport` _output_get 0)
  (`OxygenProgressBar.StartOxygenDecrease` _output_get)
  (`self.Set Oxygen Meter References` _output_get))

(event `self.ReceiveTick`
  (params (DeltaSeconds :type "Float (single-precision)"))
  (bind _returnvalue (`GameplayStatics.GetPlayerCameraManager` 0))
  (bind _returnvalue_2 (<= (`ProgressBar.Percent` (`OxygenProgressBar.OxygenBar` (`self.Oxygen Meter`))) 0.0))
  (if (and (not (`self.Dying`)) _returnvalue_2)
    (set `self.Dying` true)
    (`PlayerCameraManager.StopCameraFade` _returnvalue)
    (`PlayerCameraManager.StartCameraFade` :`self` _returnvalue :`ToAlpha` 1.0 :`Duration` 1.5 :`bShouldFadeAudio` true :`bHoldWhenFinished` true)
    (`KismetSystemLibrary.Delay` 1.5)
    (if _returnvalue_2
      (`GameplayStatics.OpenLevel` "Level_1")
      (else
        (set `self.Dying` false)
        (`PlayerCameraManager.StopCameraFade` _returnvalue)
        (`PlayerCameraManager.StartCameraFade` :`self` _returnvalue :`FromAlpha` 1.0 :`Duration` 1.5 :`bShouldFadeAudio` true)))))