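; LevelHook is a level helper Blueprint that detects desktop or VR play and exposes the player to other objects.
; On BeginPlay it caches the FirstPersonCharacter, or the VRPawn if none exists, then fades the camera in from full opacity.
; Getters return the mode, the active player and a respawn point fixed at the origin.
; Another function passes an oxygen meter reference to every OxygenTankBP's InteractableOxygenTank component.
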(event `self.ReceiveBeginPlay`
  (bind _returnvalue (`GameplayStatics.GetPlayerCameraManager` 0))
  ;[1 1 1] Set up player references
  (bind _returnvalue_2 (`GameplayStatics.GetActorOfClass` "/Game/FirstPersonBP/Blueprints/FirstPersonCharacter.FirstPersonCharacter_C"))
  (set `self.Desktop Player` _returnvalue_2)
  (bind _output_get (set `self.Is Desktop` (`KismetSystemLibrary.IsValid` _returnvalue_2)))
  (if (not _output_get)
    (bind _returnvalue_3 (`GameplayStatics.GetActorOfClass` "/Game/VRTemplate/Blueprints/VRPawn.VRPawn_C"))
    (set `self.VR Player` _returnvalue_3))
  (`PlayerCameraManager.StopCameraFade` _returnvalue)
  (`PlayerCameraManager.StartCameraFade` :`self` _returnvalue :`FromAlpha` 1.0 :`Duration` 1.5 :`bShouldFadeAudio` true))

(fn `Get Player Actor`
  (returns (Actor :type "Actor Object Reference"))
  (if (`self.Is Desktop`)
    (return (`self.Desktop Player`))
    (else
      (return (`self.VR Player`)))))

(fn `Get Player Pawn`
  (returns (Pawn :type "Pawn Object Reference"))
  (if (`self.Is Desktop`)
    (return (`self.Desktop Player`))
    (else
      (return (`self.VR Player`)))))

(fn `Get Respawn Point`
  (returns (Position :type "Vector Structure"))
  (return (0.0 0.0 0.0)))

(fn `Is Desktop Mode`
  (returns (`Is Desktop` :type Boolean))
  (return (`self.Is Desktop`)))

(fn `Set Oxygen Meter References`
  (params (`Meter Reference` :type "/Game/Oxygen/OxygenMeter Object Reference"))
  (bind _outactors (`GameplayStatics.GetAllActorsOfClass` "/Game/Oxygen/OxygenTankBP.OxygenTankBP_C"))
  (for (_array_element _array_index) _outactors
    (`/Game/Blueprints/InteractableComponents/InteractableOxygenTank.SetMeterRef` (`Actor.GetComponentByClass` _array_element "/Game/Blueprints/InteractableComponents/InteractableOxygenTank.InteractableOxygenTank_C") `Meter Reference`)
    (`KismetSystemLibrary.PrintString` "added a ref")))