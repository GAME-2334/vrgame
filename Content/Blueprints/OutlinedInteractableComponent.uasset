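; Actor component that toggles an outline highlight on its owner's meshes, named for use on interactables.
; On BeginPlay it fills MeshesToHighlight with all of the owner's static mesh components if the list is empty.
; StartOutlining and StopOutlining switch Render Custom Depth on and off for each listed mesh; the outline rendering itself is not in this Blueprint.
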(event `self.ReceiveBeginPlay`
  (if (not (> (`KismetArrayLibrary.Array_Length` (`self.Meshes to Highlight`)) 0))
    (set `self.Meshes to Highlight` (`Actor.K2_GetComponentsByClass` (`self.GetOwner`) "/Script/Engine.StaticMeshComponent"))))

(event `self.StartOutlining`
  (for _array_element (`self.Meshes to Highlight`)
    (`PrimitiveComponent.SetRenderCustomDepth` _array_element true)))

(event `self.StopOutlining`
  (for _array_element (`self.Meshes to Highlight`)
    (`PrimitiveComponent.SetRenderCustomDepth` _array_element false)))