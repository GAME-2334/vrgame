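; Level hook for the second level that sets up the oxygen survival mechanic and hands the player the flashlight.
; On BeginPlay it creates an OxygenMeter, shows it in the viewport on desktop or on the VR player's widget, then starts depletion and shares the reference.
; Tick handles desktop-only death: empty oxygen fades out, then opens Level_1 unless oxygen recovered during the fade, which fades back in.
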(event `self.ReceiveBeginPlay`
  (bind _vr_player (`self.VR Player`))
  (bind _oxygen_meter (`self.Oxygen Meter`))
  (`parent.ReceiveBeginPlay`)
  (bind _returnvalue (`|GenericCreateObject` "/Game/Oxygen/OxygenMeter.OxygenMeter_C" self))
  (set `self.Oxygen Meter` _returnvalue)
  (if (`self.Is Desktop`)
    (`/Game/FirstPersonBP/Blueprints/FirstPersonCharacter.PickedUpFlashLight` (`self.Desktop Player`))
    (`UserWidget.AddToViewport` _oxygen_meter 0)
    (else
      (`/Game/VRTemplate/Blueprints/VRPawn.PickedUpFlashLight` _vr_player)
      (`/Game/VRTemplate/Blueprints/VRPawn.Set O2 Visibility` _vr_player true)
      (bind _widget (`/Game/VRTemplate/Blueprints/VRPawn.Get Widget Reference` _vr_player))
      (`WidgetComponent.SetWidget` _widget _oxygen_meter)))
  (`OxygenProgressBar.StartOxygenDecrease` _oxygen_meter)
  (`self.Set Oxygen Meter References` _oxygen_meter))

(event `self.ReceiveTick`
  (params (DeltaSeconds :type "Float (single-precision)"))
  (bind _returnvalue (`GameplayStatics.GetPlayerCameraManager` 0))
  (bind _returnvalue_2 (<= (`ProgressBar.Percent` (`OxygenProgressBar.OxygenBar` (`self.Oxygen Meter`))) 0.0))
  (if (and (not (`self.Dying`)) _returnvalue_2 (`self.Is Desktop`))
    (set `self.Dying` true)
    (`PlayerCameraManager.StopCameraFade` _returnvalue)
    (`PlayerCameraManager.StartCameraFade` :`self` _returnvalue :`ToAlpha` 1.0 :`Duration` 1.5 :`bShouldFadeAudio` true :`bHoldWhenFinished` true)
    (`KismetSystemLibrary.Delay` 1.5)
    (if _returnvalue_2
      (`GameplayStatics.OpenLevel` "Level_1")
      (else
        (set `self.Dying` false)
        (`PlayerCameraManager.StopCameraFade` _returnvalue)
        (`PlayerCameraManager.StartCameraFade` :`self` _returnvalue :`FromAlpha` 1.0 :`Duration` 1.5 :`bShouldFadeAudio` true)))))