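; CreditsCamera is a camera actor that presents an animated logo, apparently for the credits.
; On BeginPlay it takes the player's view, holds a camera fade for a second, then reclaims the view in case a pawn took control and fades in.
; Tick accumulates time to linearly sweep the logo along a direction, and drives a dynamic material's Opacity parameter from one to zero between the configured fade times.
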(event `self.ReceiveBeginPlay`
  (bind _returnvalue (`GameplayStatics.GetPlayerController` 0))
  (bind _returnvalue_2 (`GameplayStatics.GetPlayerCameraManager` 0))
  (`PlayerController.SetViewTargetWithBlend` _returnvalue self 0.0 "VTBlend_Linear" 0.0 false)
  (`PlayerCameraManager.StartCameraFade` :`self` _returnvalue_2 :`FromAlpha` 1.0 :`ToAlpha` 1.0 :`Duration` 1.0 :`bHoldWhenFinished` true)
  (`KismetSystemLibrary.Delay` 1.0)
  (`PlayerController.SetViewTargetWithBlend` _returnvalue self 0.0 "VTBlend_Linear" 0.0 false) ; Set active again in case a pawn assumed control
  (`PlayerCameraManager.StartCameraFade` :`self` _returnvalue_2 :`FromAlpha` 1.0 :`Duration` 5.0)
  (bind _returnvalue_3 (`PrimitiveComponent.CreateDynamicMaterialInstance` (`self.Logo`) 0 "/Game/Materials/Logo.Logo" "None"))
  (set `self.Logo Material` _returnvalue_3))

(event `self.ReceiveTick`
  (params (DeltaSeconds :type "Float (single-precision)"))
  (bind _logo_fade_start_time (`self.Logo Fade Start Time`))
  (bind _logo_material (`self.Logo Material`))
  (bind _output_get (set `self.Time` (+ DeltaSeconds (`self.Time`))))
  (if (< _output_get (`self.Logo Sweep Time`))
    (`SceneComponent.K2_SetRelativeLocation` (`self.Logo`) (* (`self.Logo Sweep Direction`) (* (/ (`self.Time`) (`self.Logo Sweep Time`)) (`self.Logo Sweep End`))) false false))
  (if true
    (`/Engine/EditorBlueprintResources/StandardMacros.IsValid` _logo_material
      (:`Is Valid`
        (`MaterialInstanceDynamic.SetScalarParameterValue` _logo_material "Opacity" (`KismetMathLibrary.FClamp` (- 1.0 (/ (- (`self.Time`) _logo_fade_start_time) (- (`self.Logo Fade End Time`) _logo_fade_start_time)))))))))

(fn `UserConstructionScript`)