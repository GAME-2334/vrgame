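; Interactable oxygen tank that refills the player's oxygen meter when its interact override or BeginFilling event fires.
; The level Blueprint is expected to supply the meter widget reference through SetMeterRef, with a top-level widget search and cast as backup.
; Filling runs by the per-tank amount, then after a two-second delay stops and restarts oxygen decrease.
; The overlap-exit stop logic is disconnected and Tick is disabled.
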(event `SetMeterRef`
  (params (NewParam :type "/Game/Oxygen/OxygenMeter Object Reference"))
  ;[1 1 1] level blueprint sets everybody's meter ref after creating the meter.
  (set `self.Oxygen Progress Meter Ref` NewParam)
  (`KismetSystemLibrary.PrintString` "My ref was set"))

(event `FindOxygenMeterRef`
  ;[1 1 1] If the level blueprint did not set it, on this instance blueprint search for the oxygen meter. It is set on the level blueprint on play to be faster, but this is a backup.
  (bind _foundwidgets (`WidgetBlueprintLibrary.GetAllWidgetsOfClass` "/Script/vrgame.OxygenProgressBar"))
  (bind _output (`|GetArrayItem` _foundwidgets))
  (`KismetSystemLibrary.PrintString` (`KismetStringLibrary.Concat_StrStr` "Found Oxygen Meter Viewport Widget" (`KismetSystemLibrary.GetDisplayName` _output)))
  (bind _asoxygen_meter (cast `/Game/Oxygen/OxygenMeter` _output))
  (set `self.Oxygen Progress Meter Ref` _asoxygen_meter)
  (`self.fill_oxygen_bp`))

(event `self.InteractOverride`
  (`KismetSystemLibrary.PrintString` "adding oxygen now!!")
  ;[1 1 1] On overlap, try to fill the oxygen meter
  (if (`KismetSystemLibrary.IsValid` (`self.Oxygen Progress Meter Ref`)) :!label _label
    (`self.fill_oxygen_bp`)
    (else
      (`self.FindOxygenMeterRef`))))

(event `Begin Filling`
  ;[1 1 1] On overlap, try to fill the oxygen meter
  (goto _label))

(event `fill_oxygen_bp`
  (bind _oxygen_progress_meter_ref (`self.Oxygen Progress Meter Ref`))
  (`OxygenProgressBar.StartFillingOxygen` (`self.Oxygen Progress Meter Ref`) (`self.Amount To Fill Per Tank`))
  (`KismetSystemLibrary.Delay` 2.0)
  (`OxygenProgressBar.StopFillingOxygen` _oxygen_progress_meter_ref)
  (`OxygenProgressBar.StartOxygenDecrease` _oxygen_progress_meter_ref))