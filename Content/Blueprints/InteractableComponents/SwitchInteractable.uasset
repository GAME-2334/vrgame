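; Switch interactable component that starts a linked door lock after being used three times.
; Each accepted interaction increments a counter and blocks further use, reopening after a short delay while the count is below the threshold.
; On reaching the threshold it calls StartTick on the BPWBDoorLock2 reference and stays locked out, with debug prints reporting progress.
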(event `self.InteractOverride`
  (bind _counter (`self.counter`))
  (if (not (`self.InteractedWith`))
    (set `self.InteractedWith` true)
    (bind _result (`/Engine/EditorBlueprintResources/StandardMacros.IncrementFloat` _counter)
      (:`  `
        (if (>= _counter 3.0)
          (`/Game/World_Builder/World_BluePrints/BP_WB_DoorLock_1.StartTick` (`self.BP_WB_DoorLock_2`))
          (`KismetSystemLibrary.PrintString` "am starting")
          (else
            (`KismetSystemLibrary.PrintString` (`KismetStringLibrary.Conv_DoubleToString` _result))
            (`KismetSystemLibrary.Delay` 6.0)
            (set `self.InteractedWith` false)))))))