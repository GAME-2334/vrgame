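; An interactable component for an elevator door that slides its owning actor open and closes it automatically.
; Interacting while closed and unlocked plays a sliding sound, targets an offset position, then restores the original target after a delay.
; Tick lerps toward the target by a fixed per-frame alpha, snaps when close and clears the open flag once back home.
; Overlapping one trigger volume locks the door; the other unlocks it.
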(event `self.ReceiveBeginPlay`
  (add `Actor.OnActorBeginOverlap` (`self.TriggerVolume`) (delegate `CustomEvent_0`))
  (add `Actor.OnActorBeginOverlap` (`self.TriggerVolume2`) (delegate `CustomEvent_1`))
  (`parent.ReceiveBeginPlay`)
  (bind _output_get (set `self.Target Position` (`Actor.K2_GetActorLocation` (`self.GetOwner`))))
  (set `self.Old Position` _output_get))

(event `CustomEvent_0`
  (params (OverlappedActor :type "Actor Object Reference") (OtherActor :type "Actor Object Reference"))
  (set `self.Is Locked` true))

(event `self.ReceiveTick`
  (params (DeltaSeconds :type "Float (single-precision)"))
  (bind _returnvalue (`self.GetOwner`))
  (bind _target_position (`self.Target Position`))
  (bind _returnvalue_2 (`Actor.K2_GetActorLocation` _returnvalue))
  (`parent.ReceiveTick` DeltaSeconds)
  (if (< (`KismetMathLibrary.Vector_Distance` (`self.Target Position`) _returnvalue_2) 1.0)
    (`Actor.K2_SetActorLocation` _returnvalue _target_position false false)
    (if (== _target_position (`self.Old Position`))
      (set `self.Is Open` false))
    (else
      (`Actor.K2_SetActorLocation` _returnvalue (`KismetMathLibrary.VLerp` _returnvalue_2 _target_position (`self.Open Speed`)) false false))))

(event `CustomEvent_1`
  (params (OverlappedActor :type "Actor Object Reference") (OtherActor :type "Actor Object Reference"))
  (set `self.Is Locked` false))

(event `self.InteractOverride`
  (bind _returnvalue (`Actor.K2_GetActorLocation` (`self.GetOwner`)))
  (if (`self.Is Open`)
    _
    (elif (not (`self.Is Locked`))
      (`GameplayStatics.PlaySoundAtLocation` (`self.slidingsound`) _returnvalue (struct) 1.0 1.0 0.0 null null null)
      (set `self.Is Open` true)
      (set `self.Old Position` _returnvalue)
      (set `self.Target Position` (+ _returnvalue (`self.Open Offset`)))
      (`KismetSystemLibrary.Delay` (`self.Open Time`))
      (set `self.Target Position` (`self.Old Position`)))))