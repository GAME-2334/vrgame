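; Interactable door switch that must be used three times before it starts its linked Door.
; InteractOverride ignores input while locked or while the Door is dropping or opening, and otherwise advances a counter.
; Early presses step the plane's countdown material and briefly show red light and screen during a delay lockout.
; The final press stays locked until SwitchReset restores the counter, display and Door.
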(event `SwitchReset`
  (set `self.counter` 0)
  (set `self.InteractedWith` false)
  (`PrimitiveComponent.SetMaterial` (`/Game/World_Builder/World_BluePrints/BP_WB_DoorSwitchRegular.Plane` (`self.DoorSwitch`)) 0 "/Game/World_Builder/WB_Materials/3_Mat.3_Mat")
  (`PrimitiveComponent.SetMaterial` (`/Game/World_Builder/World_BluePrints/BP_WB_DoorSwitchRegular.StaticMesh` (`self.DoorSwitch`)) 1 "/Game/StarterBundle/ModularScifiHallways/Materials/MI_Datapad_UI_Shipment2.MI_Datapad_UI_Shipment2")
  (`/Game/World_Builder/World_BluePrints/BP_WB_DoorLockRegular.Reset` (`self.Door`)))

(event `self.InteractOverride`
  (bind _counter (`self.counter`))
  (bind _door (`self.Door`))
  (bind _doorswitch (`self.DoorSwitch`))
  (bind _staticmesh (`/Game/World_Builder/World_BluePrints/BP_WB_DoorSwitchRegular.StaticMesh` _doorswitch))
  (bind _pointlight (`/Game/World_Builder/World_BluePrints/BP_WB_DoorSwitchRegular.PointLight` _doorswitch))
  (bind _plane (`/Game/World_Builder/World_BluePrints/BP_WB_DoorSwitchRegular.Plane` (`self.DoorSwitch`)))
  (if (`self.InteractedWith`)
    _
    (elif (not (or (`/Game/World_Builder/World_BluePrints/BP_WB_DoorLockRegular.isDropping` _door) (`/Game/World_Builder/World_BluePrints/BP_WB_DoorLockRegular.isOpening` _door)))
      (set `self.InteractedWith` true)
      (bind _result (`/Engine/EditorBlueprintResources/StandardMacros.IncrementInt` _counter)
        (:`  `
          (if (> _counter 2)
            (`/Game/World_Builder/World_BluePrints/BP_WB_DoorLockRegular.StartTick` (`self.Door`))
            (`LightComponent.SetLightColor` _pointlight (struct :`R` 0.120817 :`G` 1.0 :`A` 1.0) true)
            (`PrimitiveComponent.SetMaterial` _staticmesh 1 "/Game/StarterBundle/ModularScifiHallways/Materials/MI_Datapad_UI_Shipment2.MI_Datapad_UI_Shipment2")
            (else
              (switch `int` _result
                (:`Default`
                  _)
                (:`1`
                  (`PrimitiveComponent.SetMaterial` _plane 0 "/Game/World_Builder/WB_Materials/2_Mat.2_Mat"))
                (:`2`
                  (`PrimitiveComponent.SetMaterial` _plane 0 "/Game/World_Builder/WB_Materials/1_Mat.1_Mat")))
              (`LightComponent.SetLightColor` _pointlight (struct :`R` 1.0 :`B` 0.008024 :`A` 1.0) true)
              (`PrimitiveComponent.SetMaterial` _staticmesh 1 "/Game/StarterBundle/ModularScifiHallways/Materials/MI_Datapad_UI_Shipment.MI_Datapad_UI_Shipment")
              (`KismetSystemLibrary.Delay` 1.0)
              (set `self.InteractedWith` false)
              (`LightComponent.SetLightColor` _pointlight (struct :`R` 0.120817 :`G` 1.0 :`A` 1.0) true)
              (`PrimitiveComponent.SetMaterial` _staticmesh 1 "/Game/StarterBundle/ModularScifiHallways/Materials/MI_Datapad_UI_Shipment2.MI_Datapad_UI_Shipment2"))))))))