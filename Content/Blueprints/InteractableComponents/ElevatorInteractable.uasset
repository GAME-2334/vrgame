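; ElevatorInteractable is an interactable component that plays a scripted elevator failure and then loads Level_1.
; Its InteractOverride event runs a timed chain of delays, first setting a blinking light function on the elevator's spotlight with a camera shake and an explosion sound at the player.
; It then hides the spotlight, fades the camera and holds the fade before opening the level.
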(event `self.InteractOverride`
  (bind _spotlight (`/Game/World_Builder/World_BluePrints/BP_Elevator.SpotLight` (`self.Elevator`)))
  (`KismetSystemLibrary.Delay` 3.0)
  (`LightComponent.SetLightFunctionMaterial` _spotlight "/Game/Polar/Materials/_M_Blinking_Light_Elevator._M_Blinking_Light_Elevator")
  (`PlayerCameraManager.StartCameraShake` :`self` (`PlayerController.PlayerCameraManager` (`GameplayStatics.GetPlayerController` 0)) :`ShakeClass` "/Game/Blueprints/InteractableComponents/CameraShakeTest.CameraShakeTest_C")
  (`GameplayStatics.PlaySoundAtLocation` "/Game/Audio/Elevator_Explosion_Cue.Elevator_Explosion_Cue" (`Actor.K2_GetActorLocation` (`GameplayStatics.GetPlayerCharacter` 0)) (struct) 1.0 1.0 0.0 null null null)
  (`KismetSystemLibrary.Delay` 5.0)
  (`SceneComponent.SetVisibility` _spotlight false false)
  (`PlayerCameraManager.StartCameraFade` :`self` (`PlayerController.PlayerCameraManager` (`GameplayStatics.GetPlayerController` 0)) :`ToAlpha` 1.0 :`Duration` 3.0 :`bHoldWhenFinished` true)
  (`KismetSystemLibrary.Delay` 5.0)
  (`GameplayStatics.OpenLevel` "Level_1"))