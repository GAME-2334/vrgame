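; Interactable component for an escape switch that ends the game after repeated presses, using a counter in the InteractOverride event.
; Early presses step the DoorSwitch's countdown text material, turn its light and screen red, and lock input for a short delay.
; Once the counter passes two, it triggers camera shake, an explosion sound and a fade out, prints "Credits", then quits after a delay.
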(event `self.InteractOverride`
  (bind _counter (`self.counter`))
  (bind _doorswitch (`self.DoorSwitch`))
  (bind _textrender (`/Game/World_Builder/World_BluePrints/BP_WB_DoorSwitchEscape.TextRender` (`self.DoorSwitch`)))
  (bind _playercameramanager (`PlayerController.PlayerCameraManager` (`GameplayStatics.GetPlayerController` 0)))
  (bind _staticmesh (`/Game/World_Builder/World_BluePrints/BP_WB_DoorSwitchEscape.StaticMesh` _doorswitch))
  (bind _pointlight (`/Game/World_Builder/World_BluePrints/BP_WB_DoorSwitchEscape.PointLight` _doorswitch))
  (if (not (`self.InteractedWith`))
    (set `self.InteractedWith` true)
    (bind _result (`/Engine/EditorBlueprintResources/StandardMacros.IncrementInt` _counter)
      (:`  `
        (if (> _counter 2)
          (`LightComponent.SetLightColor` _pointlight (struct :`R` 0.120817 :`G` 1.0 :`A` 1.0) true)
          (`PrimitiveComponent.SetMaterial` _staticmesh 1 "/Game/StarterBundle/ModularScifiHallways/Materials/MI_Datapad_UI_Shipment2.MI_Datapad_UI_Shipment2")
          (`PlayerCameraManager.StartCameraShake` :`self` _playercameramanager :`ShakeClass` "/Game/Blueprints/InteractableComponents/CameraShakeTriggerBox.CameraShakeTriggerBox_C")
          (`GameplayStatics.PlaySoundAtLocation` "/Game/Audio/Elevator_Explosion_Cue.Elevator_Explosion_Cue" (`Actor.K2_GetActorLocation` (`GameplayStatics.GetPlayerCharacter` 0)) (struct) 1.0 1.0 0.0 null null null)
          (`PlayerCameraManager.StartCameraFade` :`self` _playercameramanager :`ToAlpha` 1.0 :`Duration` 6.0 :`bHoldWhenFinished` true)
          (`KismetSystemLibrary.PrintString` "Credits")
          (`KismetSystemLibrary.Delay` 10.0)
          (`KismetSystemLibrary.QuitGame` (`GameplayStatics.GetPlayerController` 0) "Quit")
          (else
            (switch `int` _result
              (:`Default`
                _)
              (:`1`
                (`PrimitiveComponent.SetMaterial` _textrender 0 "/Game/World_Builder/WB_Materials/WB_Materials/2_Mat.2_Mat"))
              (:`2`
                (`PrimitiveComponent.SetMaterial` _textrender 0 "/Game/World_Builder/WB_Materials/WB_Materials/1_Mat.1_Mat")))
            (`LightComponent.SetLightColor` _pointlight (struct :`R` 1.0 :`B` 0.008024 :`A` 1.0) true)
            (`PrimitiveComponent.SetMaterial` _staticmesh 1 "/Game/StarterBundle/ModularScifiHallways/Materials/MI_Datapad_UI_Shipment.MI_Datapad_UI_Shipment")
            (`KismetSystemLibrary.Delay` 1.0)
            (set `self.InteractedWith` false)
            (`LightComponent.SetLightColor` _pointlight (struct :`R` 0.120817 :`G` 1.0 :`A` 1.0) true)
            (`PrimitiveComponent.SetMaterial` _staticmesh 1 "/Game/StarterBundle/ModularScifiHallways/Materials/MI_Datapad_UI_Shipment2.MI_Datapad_UI_Shipment2")))))))